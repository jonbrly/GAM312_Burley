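; Player character Blueprint that sets up the player's HUD and toggles the crafting menu.
; BeginPlay creates Player_W, stores it as PlayerUI and adds it to the viewport.
; The CraftMenu input drives a FlipFlop that opens a newly created Crafting_W with mouse cursor and Game-and-UI input focus.
; The next press removes it, hides the cursor and restores game-only input.
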(event `self.ReceiveBeginPlay`
  (bind _returnvalue (`|CreateWidget` "/Game/Widgets/Player_W.Player_W_C"))
  (bind _output_get (set `self.playerUI` _returnvalue))
  (`UserWidget.AddToViewport` _output_get 0))

(event `InputAction|CraftMenu`
  (params (Key :type "Key Structure"))
  (bind _returnvalue (`GameplayStatics.GetPlayerController` 0))
  (bind _returnvalue_2 (`GameplayStatics.GetPlayerController` 0))
  ;[1 1 1] Open Crafting Menu
  (:`Pressed`
    (`/Engine/EditorBlueprintResources/StandardMacros.FlipFlop`
      (:`A`
        (bind _returnvalue_3 (`|CreateWidget` "/Game/Widgets/Crafting_W.Crafting_W_C"))
        (`UserWidget.AddToViewport` _returnvalue_3 0)
        (set `PlayerController.bShowMouseCursor` true _returnvalue_2)
        (`WidgetBlueprintLibrary.SetInputMode_GameAndUIEx` _returnvalue_2 _returnvalue_3))
      (:`B`
        (`Widget.RemoveFromParent` _returnvalue_3)
        (set `PlayerController.bShowMouseCursor` false _returnvalue)
        (`WidgetBlueprintLibrary.SetInputMode_GameOnly` _returnvalue)
        (`WidgetBlueprintLibrary.SetFocusToGameViewport`)))))

(fn `UserConstructionScript`)